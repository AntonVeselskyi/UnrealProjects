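; BP_Pickup is a coin pickup actor that adds to the player's coin count.
; On BeginPlay it caches the game state as NewGameStateBase.
; When a ThirdPersonCharacter overlaps its Sphere, it adds CoinValue to that character's Coins, passes the new total to the game state's CoinTest, then destroys itself.
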(event OnComponentBeginOverlap(Sphere)
  (params (OverlappedComponent :type Primitive%20Component%20Object%20Reference) (OtherActor :type Actor%20Object%20Reference) (OtherComp :type Primitive%20Component%20Object%20Reference) (OtherBodyIndex :type Integer) (bFromSweep :type Boolean) (SweepResult :type Hit%20Result%20Structure%20%28by%20ref%29))
  (bind _asthird_person_character (Utilities|Casting|CastToThirdPersonCharacter OtherActor))
  (bind _output_get (Variables|/Game/OpenMe/Bluprints/ThirdPersonCharacter.ThirdPersonCharacter_C|SetCoins _asthird_person_character (+ (Variables|/Game/OpenMe/Bluprints/ThirdPersonCharacter.ThirdPersonCharacter_C|GetCoins _asthird_person_character) (Variables|Default|GetCoinValue))))
  (Default|CoinTest (Variables|Default|GetGameState) _output_get)
  (Actor|DestroyActor))

(event EventBeginPlay
  (Utilities|FlowControl|Sequence
    (:then_0
      (bind _asnew_game_state_base (Utilities|Casting|CastToNewGameStateBase (Game|GetGameState)))
      (Variables|Default|SetGameState _asnew_game_state_base))))

(event Collision|EventActorBeginOverlap
  (params (OtherActor :type Actor%20Object%20Reference)))

(event EventTick
  (params (DeltaSeconds :type Float%20%28single-precision%29)))

(fn ConstructionScript)